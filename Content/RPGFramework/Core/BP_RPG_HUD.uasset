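; BP_RPG_HUD is the RPG framework's HUD Blueprint that displays the player's health, stamina, adrenaline and XP bars.
; On BeginPlay it creates a WBP_RPG_HUD widget for player controller 0, stores it and adds it to the viewport.
; Four update events each take a new percentage and forward it to the matching progress bar in that widget.
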(event `self.ReceiveBeginPlay`
  (bind _returnvalue (`|CreateWidget` "/Game/RPGFramework/Blueprints/HUD/WBP_RPG_HUD.WBP_RPG_HUD_C" (`GameplayStatics.GetPlayerController` 0)))
  (bind _output_get (set `self.HUD` _returnvalue))
  (`UserWidget.AddToViewport` _output_get 0))

(event `/Game/RPGFramework/Blueprints/HUD/BPI_RPG_HUD.UpdateXPBar`
  (params (NewPercentage :type "Float (double-precision)"))
  ; Установка процента заполнения полосок атрибутов ХП, СТАМИНЫ, АДРЕНАЛИНА, XP
  (`ProgressBar.SetPercent` (`/Game/RPGFramework/Blueprints/HUD/WBP_RPG_HUD.XPBar` (`self.HUD`)) NewPercentage))

(event `/Game/RPGFramework/Blueprints/HUD/BPI_RPG_HUD.UpdateAdrenalineBar`
  (params (NewPercentage :type "Float (double-precision)"))
  ; Установка процента заполнения полосок атрибутов ХП, СТАМИНЫ, АДРЕНАЛИНА, XP
  (`ProgressBar.SetPercent` (`/Game/RPGFramework/Blueprints/HUD/WBP_RPG_HUD.AdrenalineBar` (`self.HUD`)) NewPercentage))

(event `/Game/RPGFramework/Blueprints/HUD/BPI_RPG_HUD.UpdateStaminaBar`
  (params (NewPercentage :type "Float (double-precision)"))
  ; Установка процента заполнения полосок атрибутов ХП, СТАМИНЫ, АДРЕНАЛИНА, XP
  (`ProgressBar.SetPercent` (`/Game/RPGFramework/Blueprints/HUD/WBP_RPG_HUD.StaminaBar` (`self.HUD`)) NewPercentage))

(event `/Game/RPGFramework/Blueprints/HUD/BPI_RPG_HUD.UpdateHealthBar`
  (params (NewPercentage :type "Float (double-precision)"))
  ; Установка процента заполнения полосок атрибутов ХП, СТАМИНЫ, АДРЕНАЛИНА, XP
  (`ProgressBar.SetPercent` (`/Game/RPGFramework/Blueprints/HUD/WBP_RPG_HUD.HealthBar` (`self.HUD`)) NewPercentage))

(fn `UserConstructionScript`)