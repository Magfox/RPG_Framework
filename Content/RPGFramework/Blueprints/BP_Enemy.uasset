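; BP_Enemy is the RPG framework's enemy Blueprint, adding a health bar display on top of inherited health and death logic.
; On a health change it calls the parent, shows the HUD widget component and passes the current health percentage to the widget's health bar.
; On death it calls the parent, then hides the HUD.
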(event `self.OnHealthChanged`
  (params (DeltaValue :type "Float (single-precision)") (Causer :type "Actor Object Reference"))
  ; Виджет здоровья
  (`parent.OnHealthChanged` DeltaValue Causer)
  (`SceneComponent.SetVisibility` (`self.HUD`) true true)
  (message `/Game/RPGFramework/Blueprints/HUD/BPI_EnemyHUD.UpdateHealthBar` (`WidgetComponent.GetWidget` (`self.HUD`)) (`self.F_GetHealthPercentage`)))

(event `self.OnDead`
  ; Смерть
  (`parent.OnDead`)
  (`SceneComponent.SetVisibility` (`self.HUD`) false false))

(fn `UserConstructionScript`
  (`parent.UserConstructionScript`))