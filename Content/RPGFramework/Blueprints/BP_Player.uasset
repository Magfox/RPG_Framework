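; Player character Blueprint for the RPG framework, handling Enhanced Input movement, look and melee attack, and spawning a sword attached to the hand socket on BeginPlay.
; Attribute-change and level-up events from the C++ base push health, stamina, adrenaline and XP percentages to the HUD through an interface.
; A debug graph binds keys to print attributes and trigger tagged test abilities that alter those attributes.
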(event Custom|AddInputMappings
  ;[0.138 0.2295 0.5781 0.5] Добавления контекста ввода
  (bind _asplayer_controller (Utilities|Casting|CastToPlayerController (Pawn|GetController)))
  (Utilities|IsValid (PlayerController|LocalPlayerSubsystems|GetEnhancedInputLocalPlayerSubsystem _asplayer_controller)
    (:Is%20Valid
      (Input|AddMappingContext (PlayerController|LocalPlayerSubsystems|GetEnhancedInputLocalPlayerSubsystem _asplayer_controller) "/Game/RPGFramework/Input/IMC_Standart.IMC_Standart" 0 "(bIgnoreAllPressedKeysUntilRelease=True,bForceImmediately=False,bNotifyUserSettings=False)"))))

(event Custom|SetupHUD
  ;[0 1 0.9423 0.5] Установка HUD
  (bind _asbpi_rpg_hud (Utilities|Casting|CastToBPI_RPG_HUD (HUD|GetHUD (Game|GetPlayerController 0))))
  (Variables|Default|SetRPGHud _asbpi_rpg_hud)
  (CallFunction|FUpdateBars))

(event Input|EnhancedActionEvents|EnhancedInputActionIA_Move
  (params (ActionValue :type Vector%202D%20Structure) (ElapsedSeconds :type Float%20%28double-precision%29) (TriggeredSeconds :type Float%20%28double-precision%29) (InputAction :type Input%20Action%20Object%20Reference :default "/Game/RPGFramework/Input/Actions/IA_Move.IA_Move"))
  (bind _returnvalue (Pawn|GetControlRotation :!class /Script/Engine.Pawn))
  ;[0.138 0.2295 0.5781 0.5] Базовое передвижение
  ;;[0.15 0.15 0.15 0.5] Лево право
  (Pawn|Input|AddMovementInput (Math|Vector|GetRightVector (Math|Rotator|MakeRotator (.roll _returnvalue) 0.0 (.yaw _returnvalue))) (.x ActionValue) false)
  ;;[0.15 0.15 0.15 0.5] Вперед назад
  (Pawn|Input|AddMovementInput (Math|Vector|GetForwardVector (Math|Rotator|MakeRotator 0.0 0.0 (.yaw (Pawn|GetControlRotation :!class /Script/Engine.Pawn)))) (.y ActionValue) false))

(event Input|EnhancedActionEvents|EnhancedInputActionIA_Look
  (params (ActionValue :type Vector%202D%20Structure) (ElapsedSeconds :type Float%20%28double-precision%29) (TriggeredSeconds :type Float%20%28double-precision%29) (InputAction :type Input%20Action%20Object%20Reference :default "/Game/RPGFramework/Input/Actions/IA_Look.IA_Look"))
  ;[0.138 0.2295 0.5781 0.5] Вращение камерой
  (Pawn|Input|AddControllerYawInput (.x ActionValue))
  (Pawn|Input|AddControllerPitchInput (.y ActionValue)))

(event Input|EnhancedActionEvents|EnhancedInputActionIA_Attack
  (params (ActionValue :type Boolean) (ElapsedSeconds :type Float%20%28double-precision%29) (TriggeredSeconds :type Float%20%28double-precision%29) (InputAction :type Input%20Action%20Object%20Reference :default "/Game/RPGFramework/Input/Actions/IA_Attack.IA_Attack"))
  (:Started
    (CallFunction|DoMeleeAttack)))

(event EventBeginPlay
  (|CallParentFunction)
  (CallFunction|AddInputMappings)
  (CallFunction|SetupHUD)
  (CallFunction|FEquipWeapons))

(event Collision|EventActorBeginOverlap
  (params (OtherActor :type Actor%20Object%20Reference))
  (|CallParentFunction OtherActor) ; This node is disabled and will not be called.\nDrag off pins to build functionality.
)

(event EventTick
  (params (DeltaSeconds :type Float%20%28single-precision%29))
  (|CallParentFunction DeltaSeconds) ; This node is disabled and will not be called.\nDrag off pins to build functionality.
)

(event EventOnHealthChanged
  (params (DeltaValue :type Float%20%28single-precision%29) (Causer :type Actor%20Object%20Reference))
  ;[0 1 0 0.5] Ивент об изменении здоровья (Вызов при каждом изменении)
  (Default|UpdateHealthBar (Variables|Default|GetRPGHud) (CallFunction|FGetHealthPercentage)))

(event EventOnStaminaChanged
  (params (DeltaValue :type Float%20%28single-precision%29) (Causer :type Actor%20Object%20Reference))
  ;[0 1 0 0.5] Ивент об изменении стамины (вызов при каждом изменении
  (Default|UpdateStaminaBar (Variables|Default|GetRPGHud) (CallFunction|FGetStaminaPercentage)))

(event EventOnAdrenalineChanged
  (params (DeltaValue :type Float%20%28single-precision%29) (Causer :type Actor%20Object%20Reference))
  ;[0 1 0 0.5] Ивент об изменении адреналина (вызов при каждом измении)
  (Default|UpdateAdrenalineBar (Variables|Default|GetRPGHud) (CallFunction|FGetAdrenalinePercentage)))

(event EventOnXPChanged
  (params (DeltaValue :type Float%20%28single-precision%29))
  ;[0 1 0 0.5] Ивент об изменении XP
  (Default|UpdateXPBar (Variables|Default|GetRPGHud) (CallFunction|FGetXPPercentage)))

(event EventOnCharacterLeveledUp
  ;[0 1 0 0.5] Ивент о повышении уровня персонажа
  (CallFunction|FUpdateBars))

(event Input|KeyboardEvents|DebugKeyAdd
  (params (Key :type Key%20Structure) (ActionValue :type Input%20Action%20Value%20Structure))
  ;[0.5104 0.41 0 0.5] Увеличение здоровья
  (:Pressed
    (Class|RPGCharacter|ActivateAbilitieswithTag "(GameplayTags=((TagName=\"Test.Health.Increase\")))" true) ; Кастомная функция из C++
  ))

(event Input|KeyboardEvents|DebugKeyH
  (params (Key :type Key%20Structure) (ActionValue :type Input%20Action%20Value%20Structure))
  ;[0.5104 0.41 0 0.5] Вывод атрибутов
  (:Pressed
    (Development|PrintText (Utilities|Text|FormatText "health {0} 
Maxhealth {1} 
Stamina {2} 
Max Stamina {3} 
Adrenaline {4} 
Max Adrenaline {5} 
XP {6} 
Max XP {7} 
" (Class|RPGCharacter|GetHealth) (Class|RPGCharacter|GetMaxHealth) (Class|RPGCharacter|GetStamina) (Class|RPGCharacter|GetMaxStamina) (Class|RPGCharacter|GetAdrenaline) (Class|RPGCharacter|GetMaxAdrenaline) (Class|RPGCharacter|GetExperiencePoints) (Class|RPGCharacter|GetMaxExperiencePoints)) true true "(R=0.000000,G=0.660000,B=1.000000,A=1.000000)" 1e+01)))

(event Input|KeyboardEvents|DebugKeySubtract
  (params (Key :type Key%20Structure) (ActionValue :type Input%20Action%20Value%20Structure))
  ;[0.5104 0.41 0 0.5] Уменьшение здоровья
  (:Pressed
    (Class|RPGCharacter|ActivateAbilitieswithTag "(GameplayTags=((TagName=\"Test.Health.Decrease\")))" true) ; Кастомная функция из C++
  ))

(event Input|KeyboardEvents|DebugKeyDivide
  (params (Key :type Key%20Structure) (ActionValue :type Input%20Action%20Value%20Structure))
  ;[0.5104 0.41 0 0.5] Уменьшение стамины
  (:Pressed
    (Class|RPGCharacter|ActivateAbilitieswithTag "(GameplayTags=((TagName=\"Test.Stamina.Decrease\")))" true) ; Кастомная функция из C++
  ))

(event Input|KeyboardEvents|DebugKeyMultiply
  (params (Key :type Key%20Structure) (ActionValue :type Input%20Action%20Value%20Structure))
  ;[0.5104 0.41 0 0.5] Увеличение стамины
  (:Pressed
    (Class|RPGCharacter|ActivateAbilitieswithTag "(GameplayTags=((TagName=\"Test.Stamina.Increase\")))" true) ; Кастомная функция из C++
  ))

(event Input|KeyboardEvents|DebugKeyNumPadOne
  (params (Key :type Key%20Structure) (ActionValue :type Input%20Action%20Value%20Structure))
  ;[0.5104 0.41 0 0.5] Уменьшение адреналина
  (:Pressed
    (Class|RPGCharacter|ActivateAbilitieswithTag "(GameplayTags=((TagName=\"Test.Adrenaline.Decrease\")))" true) ; Кастомная функция из C++
  ))

(event Input|KeyboardEvents|DebugKeyNumPadTwo
  (params (Key :type Key%20Structure) (ActionValue :type Input%20Action%20Value%20Structure))
  ;[0.5104 0.41 0 0.5] Увеличение адреналина
  (:Pressed
    (Class|RPGCharacter|ActivateAbilitieswithTag "(GameplayTags=((TagName=\"Test.Adrenaline.Increase\")))" true) ; Кастомная функция из C++
  ))

(event Input|KeyboardEvents|DebugKeyUp
  (params (Key :type Key%20Structure) (ActionValue :type Input%20Action%20Value%20Structure))
  ;[0.5104 0.41 0 0.5] Получение опыта персонажа
  (:Pressed
    (Class|RPGCharacter|ActivateAbilitieswithTag "(GameplayTags=((TagName=\"Test.XP.Increase\")))" true) ; Кастомная функция из C++
  ))

(fn ConstructionScript
  (|CallParentFunction))

(fn FUpdateBars
  ;[0.15 0.15 0.15 0.5] Обновляем % прогресс баров
  (Default|UpdateHealthBar (Variables|Default|GetRPGHud) (CallFunction|FGetHealthPercentage))
  (Default|UpdateStaminaBar (Variables|Default|GetRPGHud) (CallFunction|FGetStaminaPercentage))
  (Default|UpdateAdrenalineBar (Variables|Default|GetRPGHud) (CallFunction|FGetAdrenalinePercentage))
  (Default|UpdateXPBar (Variables|Default|GetRPGHud) (CallFunction|FGetXPPercentage)))

(fn FEquipWeapons
  (Utilities|FlowControl|Sequence
    (:then_0
      (bind _returnvalue (Game|SpawnActorfromClass "/Game/RPGFramework/Blueprints/Weapon/BP_Sword.BP_Sword_C" (Math|Transform|MakeTransform "0, 0, 0") "Undefined" "MultiplyWithRoot" 0 0))
      (bind _output_get (Variables|Default|SetMeleeWeapon _returnvalue))
      (Transformation|AttachComponentToComponent _output_get (Variables|Character|GetMesh) "hand_rSocket" "SnapToTarget" "SnapToTarget" "SnapToTarget" true))
    (:then_1)))