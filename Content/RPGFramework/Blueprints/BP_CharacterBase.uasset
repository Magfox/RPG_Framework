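; Base character Blueprint for an RPG framework, providing melee combo attacks, gameplay effect application and percentage getters for health, stamina, adrenaline and XP.
; A melee attack activates the ability, or if one is already active advances the combo.
; Combos require an open window and affordable GAS cost, then redirect the montage's next section using the notify's finisher or next-section name.
; Setters control combo, finisher and slow-motion flags; GetCanDoCombo returns CanDoFinisher.
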(event `/Game/RPGFramework/Blueprints/Interface/BPI_Warrior.DoMeleeAttack`
  ; Атака с комбо
  (bind _result (`self.IsUsingMelee`))
  (if _result
    (`self.F_DoNextCombo`)
    (else
      (`self.ActivateMeleeAbility` true))))

(event `/Game/RPGFramework/Blueprints/Interface/BPI_Warrior.SetCanDoSlowmotion`
  (params (Value :type Boolean))
  (set `self.DisableSlowMotion` (not Value)))

(event `/Game/RPGFramework/Blueprints/Interface/BPI_Warrior.SetCanDoFinisher`
  (params (NewCanDoFinisher :type Boolean))
  (set `self.CanDoFinisher` NewCanDoFinisher))

(event `/Game/RPGFramework/Blueprints/Interface/BPI_Warrior.SetCanDoCombo`
  (params (NewCanDoCombo :type Boolean) (NextComboNotify :type "/Game/RPGFramework/Blueprints/AnimNotify/ANS_ComboAttack Object Reference"))
  (bind _output_get (set `self.CanDoCombo` NewCanDoCombo))
  (if _output_get
    (set `self.NextComboNotify` NextComboNotify)))

(event `/Game/RPGFramework/Blueprints/Interface/BPI_Warrior.ApplyGameplatEffectByClass`
  (params (GameplayEffect :type "GameplayEffect Class Reference"))
  ; Применяем эффект
  (`self.ApplyGameplayEffect` GameplayEffect) ; c++
)

(fn `F_DoNextCombo`
  (bind _returnvalue (`SkeletalMeshComponent.GetAnimInstance` (`self.Mesh`)))
  (bind _returnvalue_2 (`AnimInstance.GetCurrentActiveMontage` _returnvalue))
  (bind _returnvalue_3 (`self.CanApplyGameplayEffect` "/Game/RPGFramework/Blueprints/Abilities/Melee/GE_Cost_Sword_Attack.GE_Cost_Sword_Attack_C")) ; c++
  (if (and (`self.CanDoCombo`) _returnvalue_3)
    ; Получаем текущую секцию монтажа и подствляем следующую из нотифая, если есть возможность выполнить финал комбо, то будет финал комбо
    (`self.NextComboNotify`
      (:`then`
        (bind _returnvalue_4 (`self.F_GetNextComboSection`))
        (`AnimInstance.Montage_SetNextSection` _returnvalue (`AnimInstance.Montage_GetCurrentSection` _returnvalue _returnvalue_2) _returnvalue_4 _returnvalue_2)
        (set `self.CanDoCombo` false)
        (set `self.DisableSlowMotion` (not (`self.CanDoFinisher`))))
      (:`else`))))

(fn `F_GetAdrenalinePercentage`
  (returns (ReturnValue :type "Float (double-precision)"))
  (return (/ (`self.GetAdrenaline`) (`self.GetMaxAdrenaline`))))

(fn `F_GetHealthPercentage`
  (returns (ReturnValue :type "Float (double-precision)"))
  (return (/ (`self.GetHealth`) (`self.GetMaxHealth`))))

(fn `F_GetNextComboSection`
  (returns (ReturnValue :type Name))
  (bind _nextcombonotify (`self.NextComboNotify`)
    (:`then`
      (bind _finishersectionname (`/Game/RPGFramework/Blueprints/AnimNotify/ANS_ComboAttack.FinisherSectionName` _nextcombonotify))
      (return (`KismetMathLibrary.SelectName` _finishersectionname (`/Game/RPGFramework/Blueprints/AnimNotify/ANS_ComboAttack.NextSectionName` _nextcombonotify) (and (`self.CanDoFinisher`) (not (`KismetStringLibrary.IsEmpty` (`KismetStringLibrary.Conv_NameToString` _finishersectionname)))))))
    (:`else`
      (return "None"))))

(fn `F_GetStaminaPercentage`
  (returns (ReturnValue :type "Float (double-precision)"))
  (return (/ (`self.GetStamina`) (`self.GetMaxStamina`))))

(fn `F_GetXPPercentage`
  (returns (ReturnValue :type "Float (double-precision)"))
  (return (/ (`self.GetExperiencePoints`) (`self.GetMaxExperiencePoints`))))

(fn `GetCanDoCombo`
  (returns (Result :type Boolean))
  (return (`self.CanDoFinisher`)))

(fn `GetCanDoFinisher`
  (returns (Result :type Boolean))
  (return (`self.CanDoFinisher`)))

(fn `GetCanDoSlowmotion`
  (returns (Result :type Boolean))
  (return (not (`self.DisableSlowMotion`))))

(fn `IsUsingMelee`
  (returns (Result :type Boolean))
  (bind _activeabilities (`self.GetActiveAbilitiesWithTags` (struct :`GameplayTags` (struct :`(TagName` "Combat.Melee"))))) ; c++
  (return (`KismetArrayLibrary.Array_IsNotEmpty` _activeabilities)))

(fn `UserConstructionScript`)